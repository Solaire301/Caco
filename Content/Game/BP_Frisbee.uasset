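; BP_Frisbee is a thrown frisbee actor that spins, flies out from its thrower, then homes back to a return target component.
; InitThrow stores the owner, target and start point, and sets velocity along the throw direction.
; Tick runs a Going/Returning state machine: a swept straight move until max distance, then an unswept VInterpTo-steered return.
; Within catch distance it casts the owner to BP_ThirdPersonCharacter, with no further action.
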(event EventBeginPlay)

(event Collision|EventActorBeginOverlap
  (params (OtherActor :type Actor%20Object%20Reference)))

(event EventTick
  (params (DeltaSeconds :type Float%20%28single-precision%29))
  (bind _output_get (Variables|Default|SetDelta%20Seconds DeltaSeconds))
  ;[0.875 0.875 0.875 0.5] Spin
  (Transformation|AddLocalRotation (Variables|Default|GetCylinder) (Math|Rotator|MakeRotator 0.0 0.0 (* _output_get (Variables|Default|GetSpinSpeed))) false false)
  (switch Utilities|FlowControl|Switch|SwitchonE_FrisbeeState (Variables|Default|GetState)
    (:NewEnumerator0
      ;[0.05882 0.05882 0.05882 0.502] Going
      (if (>= (Math|Vector|Distance(Vector) (Transformation|GetActorLocation) (Variables|Default|GetStartLocation)) (Variables|Default|GetMaxDistance))
        (Variables|Default|SetState "NewEnumerator1")
        (else
          (Transformation|SetActorLocation (+ (* (Variables|Default|GetVelocity) (Variables|Default|GetDelta%20Seconds)) (Transformation|GetActorLocation)) true false))))
    (:NewEnumerator1
      ;[0.05882 0.05882 0.05882 0.502] Returning
      (bind _output_get_2 (Variables|Default|SetTargetLocation (Transformation|GetWorldLocation (Variables|Default|GetReturnTargetComp))))
      (bind _output_get_3 (Variables|Default|SetDesiredVelocity (* (Math|Vector|Normalize (- _output_get_2 (Transformation|GetActorLocation))) (Variables|Default|GetReturnSpeed))))
      (Variables|Default|SetVelocity (Math|Interpolation|VInterpTo (Variables|Default|GetVelocity) _output_get_3 (Variables|Default|GetDelta%20Seconds) (Variables|Default|GetTurnStrength)))
      (Transformation|SetActorLocation (+ (Transformation|GetActorLocation) (* (Variables|Default|GetVelocity) (Variables|Default|GetDelta%20Seconds))) false false)
      (if (<= (Math|Vector|Distance(Vector) (Transformation|GetWorldLocation (Variables|Default|GetReturnTargetComp)) (Transformation|GetActorLocation)) (Variables|Default|GetCatchDistance))
        (Utilities|Casting|CastToBP_ThirdPersonCharacter (Variables|Default|GetOwnerActor))))))

(fn ConstructionScript)

(fn InitThrow
  (params (InOwner :type Actor%20Object%20Reference) (InRetrunTargetComp :type Scene%20Component%20Object%20Reference) (ThrowDirection :type Vector))
  (Variables|Default|SetOwnerActor InOwner)
  (Variables|Default|SetReturnTargetComp InRetrunTargetComp)
  (Variables|Default|SetStartLocation (Transformation|GetActorLocation))
  (Variables|Default|SetState "NewEnumerator0")
  (bind _output_get (Variables|Default|SetNormDirection (Math|Vector|Normalize ThrowDirection)))
  (Variables|Default|SetVelocity (* _output_get (Variables|Default|GetSpeed))))