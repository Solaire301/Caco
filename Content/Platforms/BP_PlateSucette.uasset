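; BP_PlateSucette is a platform that makes the player slippery, like ice, while they are on it.
; When a BP_ThirdPersonCharacter enters its Box, it overrides CharacterMovement with negative ground friction, weak braking and low acceleration.
; Leaving the Box writes hardcoded normal movement values back rather than restoring the character's previous settings.
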(event OnComponentBeginOverlap(Box)
  (params (OverlappedComponent :type Primitive%20Component%20Object%20Reference) (OtherActor :type Actor%20Object%20Reference) (OtherComp :type Primitive%20Component%20Object%20Reference) (OtherBodyIndex :type Integer) (bFromSweep :type Boolean) (SweepResult :type Hit%20Result%20Structure%20%28by%20ref%29))
  (bind _asbp_third_person_character (Utilities|Casting|CastToBP_ThirdPersonCharacter OtherActor))
  (Utilities|FlowControl|Sequence
    (:then_0
      (Variables|/Script/Engine.CharacterMovementComponent|SetGroundFriction (Variables|/Script/Engine.Character|GetCharacterMovement _asbp_third_person_character) -5.0))
    (:then_1
      (Variables|/Script/Engine.CharacterMovementComponent|SetBrakingDecelerationWalking (Variables|/Script/Engine.Character|GetCharacterMovement _asbp_third_person_character) 5e+01))
    (:then_2
      (Variables|/Script/Engine.CharacterMovementComponent|SetMaxAcceleration (Variables|/Script/Engine.Character|GetCharacterMovement _asbp_third_person_character) 5e+02))
    (:then_3
      (Variables|/Script/Engine.CharacterMovementComponent|SetBrakingFrictionFactor (Variables|/Script/Engine.Character|GetCharacterMovement _asbp_third_person_character) 0.0))
    (:then_4
      (Variables|/Script/Engine.CharacterMovementComponent|SetbUseSeparateBrakingFriction (Variables|/Script/Engine.Character|GetCharacterMovement _asbp_third_person_character) true))))

(event OnComponentEndOverlap(Box)
  (params (OverlappedComponent :type Primitive%20Component%20Object%20Reference) (OtherActor :type Actor%20Object%20Reference) (OtherComp :type Primitive%20Component%20Object%20Reference) (OtherBodyIndex :type Integer))
  (bind _asbp_third_person_character (Utilities|Casting|CastToBP_ThirdPersonCharacter OtherActor))
  (Utilities|FlowControl|Sequence
    (:then_0
      (Variables|/Script/Engine.CharacterMovementComponent|SetGroundFriction (Variables|/Script/Engine.Character|GetCharacterMovement _asbp_third_person_character) 8.0))
    (:then_1
      (Variables|/Script/Engine.CharacterMovementComponent|SetBrakingDecelerationWalking (Variables|/Script/Engine.Character|GetCharacterMovement _asbp_third_person_character) 2e+03))
    (:then_2
      (Variables|/Script/Engine.CharacterMovementComponent|SetMaxAcceleration (Variables|/Script/Engine.Character|GetCharacterMovement _asbp_third_person_character) 2.5e+03))
    (:then_3
      (Variables|/Script/Engine.CharacterMovementComponent|SetBrakingFrictionFactor (Variables|/Script/Engine.Character|GetCharacterMovement _asbp_third_person_character) 1.0))
    (:then_4
      (Variables|/Script/Engine.CharacterMovementComponent|SetbUseSeparateBrakingFriction (Variables|/Script/Engine.Character|GetCharacterMovement _asbp_third_person_character) false))))

(event EventBeginPlay)

(event EventTick
  (params (DeltaSeconds :type Float%20%28single-precision%29)))

(fn ConstructionScript)