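; BP_PlateBiscuit is a timed platform that destroys itself after the player character touches it.
; A Box overlap with BP_ThirdPersonCharacter starts a timer, which Tick advances by delta time scaled by Multiplicator.
; The actor is destroyed when the value reaches its final threshold; the three intermediate threshold checks are empty, and nothing stops or resets the countdown.
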(event OnComponentBeginOverlap(Box)
  (params (OverlappedComponent :type Primitive%20Component%20Object%20Reference) (OtherActor :type Actor%20Object%20Reference) (OtherComp :type Primitive%20Component%20Object%20Reference) (OtherBodyIndex :type Integer) (bFromSweep :type Boolean) (SweepResult :type Hit%20Result%20Structure%20%28by%20ref%29))
  (Utilities|Casting|CastToBP_ThirdPersonCharacter OtherActor)
  (Variables|Default|SetStartTimer true))

(event EventBeginPlay)

(event EventTick
  (params (DeltaSeconds :type Float%20%28single-precision%29))
  (if (Variables|Default|GetStartTimer)
    (bind _output_get (Variables|Default|SetValue (+ (* DeltaSeconds (Variables|Default|GetMultiplicator)) (Variables|Default|GetValue))))
    (Utilities|FlowControl|Sequence
      (:then_0
        (if (>= _output_get 25.0)
          _))
      (:then_1
        (if (>= _output_get 5e+01)
          _))
      (:then_2
        (if (>= _output_get 75.0)
          _))
      (:then_3
        (if (>= _output_get 1e+02)
          (Actor|DestroyActor))))))

(fn ConstructionScript)