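; A thrown frisbee projectile that flies out from the player, damages what it hits, and returns like a boomerang to be caught.
; InitThrow stores the owner and return component and sets the launch velocity; Tick spins the mesh and runs a Going/Returning state machine.
; It turns back at max range or on a Box hit, then homes via VInterpTo-steered velocity without sweep.
; Within catch distance it notifies BP_ThirdPersonCharacter and destroys itself.
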(event OnComponentHit(Box)
  (params (HitComponent :type Primitive%20Component%20Object%20Reference) (OtherActor :type Actor%20Object%20Reference) (OtherComp :type Primitive%20Component%20Object%20Reference) (NormalImpulse :type Vector :default "0, 0, 0") (Hit :type Hit%20Result%20Structure%20%28by%20ref%29))
  (if (== (Variables|Default|GetState) 0)
    (Variables|Default|SetState "NewEnumerator1")
    (Game|Damage|ApplyDamage OtherActor (Variables|Default|GetBase%20Damage) 0 0)))

(event EventBeginPlay)

(event Collision|EventActorBeginOverlap
  (params (OtherActor :type Actor%20Object%20Reference)))

(event EventTick
  (params (DeltaSeconds :type Float%20%28single-precision%29))
  (bind _output_get (Variables|Default|SetDelta%20Seconds DeltaSeconds))
  ;[0.875 0.875 0.875 0.5] Spin
  (Transformation|AddLocalRotation (Variables|Default|GetCylinder) (Math|Rotator|MakeRotator 0.0 0.0 (* _output_get (Variables|Default|GetSpinSpeed))) false false)
  (switch Utilities|FlowControl|Switch|SwitchonE_FrisbeeState (Variables|Default|GetState)
    (:NewEnumerator0
      ;[0.05882 0.05882 0.05882 0.502] Going
      (if (>= (Math|Vector|Distance(Vector) (Transformation|GetActorLocation) (Variables|Default|GetStartLocation)) (Variables|Default|GetMaxDistance))
        (Variables|Default|SetState "NewEnumerator1")
        (else
          (Transformation|SetActorLocation (+ (* (Variables|Default|GetVelocity) (Variables|Default|GetDelta%20Seconds)) (Transformation|GetActorLocation)) true false))))
    (:NewEnumerator1
      ;[0.05882 0.05882 0.05882 0.502] Returning
      (bind _output_get_2 (Variables|Default|SetTargetLocation (Transformation|GetWorldLocation (Variables|Default|GetReturnTargetComp))))
      (bind _output_get_3 (Variables|Default|SetDesiredVelocity (* (Math|Vector|Normalize (- _output_get_2 (Transformation|GetActorLocation))) (Variables|Default|GetReturnSpeed))))
      (Variables|Default|SetVelocity (Math|Interpolation|VInterpTo (Variables|Default|GetVelocity) _output_get_3 (Variables|Default|GetDelta%20Seconds) (Variables|Default|GetTurnStrength)))
      (Transformation|SetActorLocation (+ (Transformation|GetActorLocation) (* (Variables|Default|GetVelocity) (Variables|Default|GetDelta%20Seconds))) false false)
      (if (<= (Math|Vector|Distance(Vector) (Transformation|GetWorldLocation (Variables|Default|GetReturnTargetComp)) (Transformation|GetActorLocation)) (Variables|Default|GetCatchDistance))
        (bind _asbp_third_person_character (Utilities|Casting|CastToBP_ThirdPersonCharacter (Variables|Default|GetOwnerActor)))
        (Default|OnFrisbeeCaught _asbp_third_person_character)
        (Actor|DestroyActor)))))

(fn ConstructionScript)

(fn InitThrow
  (params (InOwner :type Actor%20Object%20Reference) (InRetrunTargetComp :type Scene%20Component%20Object%20Reference) (ThrowDirection :type Vector))
  (Development|PrintString "InitOK")
  (Variables|Default|SetOwnerActor InOwner)
  (Variables|Default|SetReturnTargetComp InRetrunTargetComp)
  (Variables|Default|SetStartLocation (Transformation|GetActorLocation))
  (Variables|Default|SetState "NewEnumerator0")
  (bind _output_get (Variables|Default|SetNormDirection (Math|Vector|Normalize ThrowDirection 0.001)))
  (bind _output_get_2 (Variables|Default|SetVelocity (* _output_get (Variables|Default|GetSpeed))))
  (Development|PrintString (Utilities|String|ToString(Vector) _output_get_2)))